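; EglabMLMgr is an ML manager Blueprint that links the game to a Python agent through a TensorflowComponent, using pause-stepped control.
; It holds the game paused until the script starts, then periodically pauses to send observation, reward and done as JSON.
; Returned results become AI input for move, rotation and weapon change, and unpause the game.
; Backend disconnection also unpauses the game.
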(event `self.ReceiveBeginPlay`
  (set `self.ScriptStarted` false)
  (set `self.hasValue` false)
  (`GameplayStatics.SetGamePaused` true))

(event `self.TensorflowComponent.OnScriptStarted`
  (params (ScriptName :type String))
  (set `self.ScriptStarted` true)
  (`GameplayStatics.SetGamePaused` false))

(event `self.ReceiveTick`
  (params (DeltaSeconds :type "Float (single-precision)"))
  (set `self.deley` (+ DeltaSeconds (`self.deley`)))
  (if (>= (`self.deley`) 0.1)
    (set `self.deley` 0.0)
    (if (== (`self.ScriptStarted`) true)
      (bind (_observation _reward _done) (`self.GetAIInputResult`))
      (bind _returnvalue (`SIOJsonObject.ConstructJsonObject`))
      (`SIOJsonObject.SetNumberArrayField` _returnvalue "observation" _observation)
      (`SIOJsonObject.SetNumberField` _returnvalue "reward" _reward)
      (`SIOJsonObject.SetBoolField` _returnvalue "done" _done)
      (`GameplayStatics.SetGamePaused` true)
      (`MachineLearningRemoteComponent.SendSIOJsonInput` (`self.TensorflowComponent`) (`SIOJLibrary.Conv_JsonObjectToJsonValue` _returnvalue) "on_json_input"))
    (elif (== (`self.hasValue`) true)
      (bind _returnvalue_2 (`SIOJLibrary.Conv_JsonValueToJsonObject` (stale `self.TensorflowComponent.OnInputScriptResult` ResultData)))
      (`self.SetAIInput` (`|MakeArray` (`KismetMathLibrary.FTrunc` (`SIOJsonObject.GetNumberField` _returnvalue_2 "move")) (`KismetMathLibrary.FTrunc` (`SIOJsonObject.GetNumberField` _returnvalue_2 "rotation")) (`KismetMathLibrary.FTrunc` (`SIOJsonObject.GetNumberField` _returnvalue_2 "change_weapon"))) :!label _label)
      (`GameplayStatics.SetGamePaused` false))))

(event `self.TensorflowComponent.OnInputScriptResult`
  (params (ResultData :type "SIOJsonValue Object Reference") (CallingFunctionName :type String))
  (set `self.LastInput` ResultData)
  (set `self.hasValue` true)
  (goto _label))

(event `self.TensorflowComponent.OnDisconnectedFromBackend`
  (params (Endpoint :type String))
  (`GameplayStatics.SetGamePaused` false))

(fn `UserConstructionScript`)